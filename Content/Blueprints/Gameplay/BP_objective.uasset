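; BP_objective is a chainable objective actor that shows or hides its ObjectiveMarker as the objective starts and ends.
; BeginPlay starts or ends it based on the ObjectiveTrigger flag.
; Ending calls NextObjective, which, if NextObjectiveTriggered is set, clears that flag, then starts the linked NextMarker and calls HasObjective on QuestNPC, each when valid.
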(event Custom|Objective%20Start
  (Variables|Default|SetObjective%20Trigger true)
  (Rendering|SetVisibility (Variables|Default|GetObjective_Marker) true false))

(event Custom|Objective%20End
  (Variables|Default|SetObjective%20Trigger false)
  (Rendering|SetVisibility (Variables|Default|GetObjective_Marker) false false)
  (CallFunction|NextObjective))

(event Custom|NextObjective
  (if (Variables|Default|GetNextObjectiveTriggered)
    (Variables|Default|SetNextObjectiveTriggered false)
    (Utilities|FlowControl|Sequence
      (:then_0
        (bind _nextmarker (Variables|Default|GetNextMarker)
          (:then
            (CallFunction|ObjectiveStart _nextmarker))
          (:else)))
      (:then_1
        (bind _questnpc (Variables|Default|GetQuestNPC)
          (:then
            (Default|HasObjective _questnpc))
          (:else))))))

(event EventBeginPlay
  (if (Variables|Default|GetObjective%20Trigger)
    (CallFunction|ObjectiveStart)
    (else
      (CallFunction|ObjectiveEnd))))

(event Collision|EventActorBeginOverlap
  (params (OtherActor :type Actor%20Object%20Reference)))

(event EventTick
  (params (DeltaSeconds :type Float%20%28single-precision%29)))

(fn ConstructionScript)