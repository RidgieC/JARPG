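; BP_ItemPickUp is an item actor that highlights when a BP_Character is in range and links to a BPObjective.
; Interaction box overlaps track player range and toggle the mesh's custom depth and stencil highlight.
; If ObjectiveActive is set at BeginPlay, it starts the objective and changes the stencil value.
; Otherwise, leaving the box flags the next objective, ends the current one and destroys the item, provided BPObjective is valid.
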(event OnComponentBeginOverlap(InteractionBox)
  (params (OverlappedComponent :type Primitive%20Component%20Object%20Reference) (OtherActor :type Actor%20Object%20Reference) (OtherComp :type Primitive%20Component%20Object%20Reference) (OtherBodyIndex :type Integer) (bFromSweep :type Boolean) (SweepResult :type Hit%20Result%20Structure%20%28by%20ref%29))
  (Utilities|Casting|CastToBP_Character OtherActor)
  (Variables|Default|SetPlayerIsInRange true)
  (CallFunction|InteractionStart))

(event OnComponentEndOverlap(InteractionBox)
  (params (OverlappedComponent :type Primitive%20Component%20Object%20Reference) (OtherActor :type Actor%20Object%20Reference) (OtherComp :type Primitive%20Component%20Object%20Reference) (OtherBodyIndex :type Integer))
  (Utilities|Casting|CastToBP_Character OtherActor)
  (Variables|Default|SetPlayerIsInRange false)
  (CallFunction|InteractionEnd))

(event Custom|InteractionEnd
  (Rendering|SetRenderCustomDepth (Variables|Default|GetItemMesh) false)
  (if (not (Variables|Default|GetObjectiveActive))
    (bind _bpobjective (Variables|Default|GetBPObjective)
      (:then
        (Variables|/Game/Blueprints/Gameplay/BP_objective.BP_Objective_C|SetNextObjectiveTriggered _bpobjective true)
        (Default|ObjectiveEnd _bpobjective)
        (Actor|DestroyActor))
      (:else))))

(event Custom|InteractionStart
  (bind _itemmesh (Variables|Default|GetItemMesh))
  (Rendering|SetRenderCustomDepth _itemmesh true)
  (Rendering|SetCustomDepthStencilValue _itemmesh (Variables|Default|Getvalue)))

(event Custom|HasObjective
  (Variables|Default|SetObjectiveActive true)
  (bind _bpobjective (Variables|Default|GetBPObjective)
    (:then
      (Default|ObjectiveStart _bpobjective)
      (Variables|Default|Setvalue 2))
    (:else)))

(event EventBeginPlay
  (if (Variables|Default|GetObjectiveActive)
    (CallFunction|HasObjective)))

(event Collision|EventActorBeginOverlap
  (params (OtherActor :type Actor%20Object%20Reference)))

(event EventTick
  (params (DeltaSeconds :type Float%20%28single-precision%29)))

(fn ConstructionScript)