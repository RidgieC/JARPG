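; Weather controller Blueprint that can turn the sky overcast during play.
; A one-shot timer 30 seconds after BeginPlay makes a single random roll.
; On a rare hit, a Timeline lerps the referenced sky material's zenith and horizon colors to gray; otherwise it deactivates the rain particles.
; Rain activation, cloud and light changes, and a FlipFlop toggle are unwired, and the left-click handler does nothing.
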(event Custom|Weather
  (bind _skyreference (Variables|Default|GetSkyreference))
  (bind _output (Utilities|ResolveSoftReference _skyreference))
  (bind _sky_material (Variables|/Engine/EngineSky/BP_Sky_Sphere.BP_Sky_Sphere_C|GetSky%20material _output))
  (if (== (Math|Random|RandomIntegerinRange 0 10) 1)
    (Utilities|FlowControl|Sequence
      (:then_0
        (bind _weatherchanges (Timeline|Timeline_0 Play)
          (:Update
            (Rendering|Material|SetVectorParameterValue _sky_material "Zenith Color" (Math|Color|Lerp(LinearColor) "(R=0.034046,G=0.109247,B=0.295000,A=1.000000)" "(R=0.125000,G=0.125000,B=0.125000,A=1.000000)" _weatherchanges) :!class /Script/Engine.MaterialInstanceDynamic)
            (Rendering|Material|SetVectorParameterValue _sky_material "Horizon color" (Math|Color|Lerp(LinearColor) "(R=1.979559,G=2.586644,B=3.000000,A=1.000000)" "(R=0.161458,G=0.161458,B=0.161458,A=1.000000)" _weatherchanges) :!class /Script/Engine.MaterialInstanceDynamic))))
      (:then_1
        (Utilities|FlowControl|Delay 5.0)))
    (else
      (Components|Activation|Deactivate (Variables|/Script/Engine.Emitter|GetParticleSystemComponent (Variables|Default|GetRainreference)))
      (Utilities|FlowControl|Delay 3.0))))

(event EventBeginPlay
  (Utilities|Time|SetTimerbyEvent (delegate Custom|Weather) 3e+01))

(event Input|MouseEvents|LeftMouseButton
  (params (Key :type Key%20Structure))
  (:Pressed
    (if (Utilities|IsValid (Utilities|ResolveSoftReference (Variables|Default|GetSkyreference)))
      _)))

(fn ConstructionScript)