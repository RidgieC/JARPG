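; BP_MeasurementTool is a measuring actor that builds rulers of marker actors along X, Y and Z.
; Its construction script runs three events that spawn MeasureNumber markers per axis at 100-unit steps from the root's relative transform.
; AttachActors re-attaches every stored marker to the tool after each spawn.
; A separate Cleanup event, not called here, destroys markers found through level-wide class searches, alongside array entries.
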(event Custom|SetMeasurementZ
  (bind _output_get (Variables|Default|SetCurrentTransformZ (Transformation|GetRelativeTransform (Variables|Default|GetDefaultSceneRoot))))
  (for _index (range 1 (Variables|Default|GetMeasureNumber))
    (Variables|Default|SetCurrentNumber _index)
    (bind _returnvalue (Game|SpawnActorfromClass "/Game/Blueprints/Tools/BP_MeasurementZ.BP_MeasurementZ_C" _output_get "Undefined" 0 0))
    (Utilities|Array|Add (Variables|Default|GetMeterArrayZ) _returnvalue)
    (Variables|Default|SetCurrentTransformZ (Math|Transform|MakeTransform (+ (.location (Variables|Default|GetCurrentTransformZ)) "0, 0,100.000000") (.rotation (Variables|Default|GetCurrentTransformZ)) (.scale (Variables|Default|GetCurrentTransformZ))))
    (CallFunction|AttachActors)))

(event Custom|AttachActors
  (Utilities|FlowControl|Sequence
    (:then_0
      (for _array_element (Variables|Default|GetMeterArrayZ)
        (Transformation|AttachActorToActor _array_element self "None" "KeepWorld" "SnapToTarget" "SnapToTarget" true)))
    (:then_1
      (for _array_element_2 (Variables|Default|GetMeterArrayX)
        (Transformation|AttachActorToActor _array_element_2 self "None" "KeepWorld" "SnapToTarget" "SnapToTarget" true)))
    (:then_2
      (for _array_element_3 (Variables|Default|GetMeterArrayY)
        (Transformation|AttachActorToActor _array_element_3 self "None" "KeepWorld" "SnapToTarget" "SnapToTarget" true)))))

(event Custom|Cleanup
  (bind _meterarrayx (Variables|Default|GetMeterArrayX))
  (bind _meterarrayz (Variables|Default|GetMeterArrayZ))
  (Utilities|FlowControl|Sequence
    (:then_0
      (bind _outactors (Actor|GetAllActorsOfClass "/Game/Blueprints/Tools/BP_MeasurementZ.BP_MeasurementZ_C"))
      (for (_array_element _array_index) _outactors
        (Actor|DestroyActor (Utilities|Array|Get(acopy) _meterarrayz _array_index))
        (Utilities|Array|RemoveIndex _meterarrayz (Variables|Default|GetCurrentNumber))))
    (:then_1
      (bind _outactors_2 (Actor|GetAllActorsOfClass "/Game/Blueprints/Tools/BP_MeasurementX.BP_MeasurementX_C"))
      (for (_array_element_2 _array_index_2) _outactors_2
        (Actor|DestroyActor (Utilities|Array|Get(acopy) _meterarrayx _array_index_2))
        (Utilities|Array|RemoveIndex _meterarrayx (Variables|Default|GetCurrentNumber))))
    (:then_2
      (bind _outactors_3 (Actor|GetAllActorsOfClass "/Game/Blueprints/Tools/BP_MeasurementY.BP_MeasurementY_C"))
      (for (_array_element_3 _array_index_3) _outactors_3
        (Actor|DestroyActor _array_element_3)
        (Utilities|Array|RemoveIndex (Variables|Default|GetMeterArrayY) (Variables|Default|GetCurrentNumber))))))

(event Custom|SetMeasurementX
  (bind _output_get (Variables|Default|SetCurrentTransformX (Transformation|GetRelativeTransform (Variables|Default|GetDefaultSceneRoot))))
  (for _index (range 1 (Variables|Default|GetMeasureNumber))
    (Variables|Default|SetCurrentNumber _index)
    (bind _returnvalue (Game|SpawnActorfromClass "/Game/Blueprints/Tools/BP_MeasurementX.BP_MeasurementX_C" _output_get "Undefined" 0 0))
    (Utilities|Array|Add (Variables|Default|GetMeterArrayX) _returnvalue)
    (Variables|Default|SetCurrentTransformX (Math|Transform|MakeTransform (+ (.location (Variables|Default|GetCurrentTransformX)) "100.000000, 0, 0") (.rotation (Variables|Default|GetCurrentTransformX)) (.scale (Variables|Default|GetCurrentTransformX))))
    (CallFunction|AttachActors)))

(event Custom|SetMeasurementY
  (bind _output_get (Variables|Default|SetCurrentTransformY (Transformation|GetRelativeTransform (Variables|Default|GetDefaultSceneRoot))))
  (for _index (range 1 (Variables|Default|GetMeasureNumber))
    (Variables|Default|SetCurrentNumber _index)
    (bind _returnvalue (Game|SpawnActorfromClass "/Game/Blueprints/Tools/BP_MeasurementY.BP_MeasurementY_C" _output_get "Undefined" 0 0))
    (Utilities|Array|Add (Variables|Default|GetMeterArrayY) _returnvalue)
    (Variables|Default|SetCurrentTransformY (Math|Transform|MakeTransform (+ (.location (Variables|Default|GetCurrentTransformY)) "0,100.000000, 0") (.rotation (Variables|Default|GetCurrentTransformY)) (.scale (Variables|Default|GetCurrentTransformY))))
    (CallFunction|AttachActors)))

(fn ConstructionScript
  (CallFunction|SetMeasurementZ)
  (CallFunction|SetMeasurementX)
  (CallFunction|SetMeasurementY))