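; Sword-wielding enemy character with roam, chase and attack events, a camera-facing health widget and ragdoll death that stops its AI logic.
; Hit reactions slide it away or launch it at low gravity, restoring gravity once per-tick height tracking detects the apex.
; An overlap volume compares player and enemy levels, tinting the player's Reiatsu blue or red with a pressure sound and flagging stronger enemies.
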(event OnComponentBeginOverlap(LevelDetection)
  (params (OverlappedComponent :type Primitive%20Component%20Object%20Reference) (OtherActor :type Actor%20Object%20Reference) (OtherComp :type Primitive%20Component%20Object%20Reference) (OtherBodyIndex :type Integer) (bFromSweep :type Boolean) (SweepResult :type Hit%20Result%20Structure%20%28by%20ref%29))
  ;[1 1 1] LevelDetection
  (if (== OtherActor (Variables|Default|GetBPCharacter))
    (Variables|Default|SetCanCheckLevel true)
    (CallFunction|LevelCheck)))

(event OnComponentEndOverlap(LevelDetection)
  (params (OverlappedComponent :type Primitive%20Component%20Object%20Reference) (OtherActor :type Actor%20Object%20Reference) (OtherComp :type Primitive%20Component%20Object%20Reference) (OtherBodyIndex :type Integer))
  (bind _bpcharacter (Variables|Default|GetBPCharacter))
  ;[1 1 1] LevelDetection
  (if (== _bpcharacter OtherActor)
    (Variables|/Game/Character/BP_Character.BP_Character_C|SetHighLvlEnemy _bpcharacter false)
    (Variables|Default|SetCanCheckLevel false)
    (CallFunction|LevelCheck)))

(event Custom|Roam
  ;[1 1 1] Roam and Chase
  (Variables|/Script/Engine.CharacterMovementComponent|SetMaxWalkSpeed (Variables|Character|GetCharacterMovement) 1e+02))

(event Custom|Chase
  ;[1 1 1] Roam and Chase
  (Variables|/Script/Engine.CharacterMovementComponent|SetMaxWalkSpeed (Variables|Character|GetCharacterMovement) 5e+02))

(event Custom|HitReactRKickDistance
  (bind _bpcharacter (Variables|Default|GetBPCharacter))
  (Character|LaunchCharacter (* (Math|Vector|RotateVector (Transformation|GetActorForwardVector _bpcharacter) (Math|Vector|RotatorfromAxisandAngle (Math|Vector|NegateVector (Transformation|GetActorRightVector _bpcharacter)) 8e+01)) 35.0) false false)
  (Variables|/Script/Engine.CharacterMovementComponent|SetGravityScale (Variables|Character|GetCharacterMovement) 0.2)
  (CallFunction|ResetGravity)
  (Collision|SetCollisionEnabled (Variables|Default|GetBlockPlayer) "NoCollision"))

(event Custom|CalculateLaunchHeight
  (Variables|Default|SetCurrentHeight (.z (Transformation|GetWorldLocation (Variables|Collision|GetCapsuleComponent))))
  (Variables|Default|SetNewLaunchHeight (- (Variables|Default|GetCurrentHeight) (Variables|Default|GetStartHeight)))
  (if (< (Variables|Default|GetNewLaunchHeight) (Variables|Default|GetLaunchHeight))
    (Variables|Default|SetLaunchApex true)
    (else
      (Variables|Default|SetLaunchApex false)))
  (Variables|Default|SetLaunchHeight (Variables|Default|GetNewLaunchHeight)))

(event Custom|ResetGravity
  (Timeline|HeightCheck PlayFromStart
    (:Update
      (if (Variables|Default|GetLaunchApex)
        (CallFunction|StopResetGravity)
        (Variables|/Script/Engine.CharacterMovementComponent|SetGravityScale (Variables|Character|GetCharacterMovement) 1.0)
        (Collision|SetCollisionEnabled (Variables|Default|GetBlockPlayer) "QueryAndPhysics")))))

(event Custom|StopResetGravity
  (Timeline|HeightCheck Stop
    (:Update
      (if (Variables|Default|GetLaunchApex)
        (CallFunction|StopResetGravity)
        (Variables|/Script/Engine.CharacterMovementComponent|SetGravityScale (Variables|Character|GetCharacterMovement) 1.0)
        (Collision|SetCollisionEnabled (Variables|Default|GetBlockPlayer) "QueryAndPhysics")))))

(event Custom|HitReactPunchAir
  (Development|PrintString "GotHit")
  (CallFunction|StopResetGravity)
  (Variables|/Script/Engine.CharacterMovementComponent|SetGravityScale (Variables|Character|GetCharacterMovement) 1e+01))

(event Custom|HitReactLPunchDistance
  (bind _capsulecomponent (Variables|Collision|GetCapsuleComponent))
  (Components|MoveComponentTo _capsulecomponent (Transformation|GetWorldLocation (Variables|Default|GetHitReactCrouchDistance)) (Math|Rotator|FindLookatRotation (Transformation|GetWorldLocation _capsulecomponent) (Transformation|GetWorldLocation (Variables|/Script/Engine.Character|GetCapsuleComponent (Variables|Default|GetBPCharacter)))) false false 1.5 false))

(event Custom|HitReactLKickDistance)

(event Custom|DeathLogic
  (bind _self self)
  (bind _returnvalue (AI|GetAIController _self))
  (Variables|Default|SetDead true)
  (Utilities|FlowControl|Sequence
    (:then_0
      (Utilities|FlowControl|Delay 1.0)
      (Physics|SetSimulatePhysics (Variables|Character|GetMesh) true)
      (Pawn|Components|CharacterMovement|DisableMovement (Variables|Character|GetCharacterMovement))
      (Collision|SetCollisionEnabled (Variables|Character|GetMesh) "QueryAndPhysics")
      (Collision|SetCollisionEnabled (Variables|Collision|GetCapsuleComponent) "NoCollision"))
    (:then_1
      (AI|Logic|StopLogic (Variables|/Script/AIModule.AIController|GetBrainComponent _returnvalue) "Death")
      (Pawn|UnPossess _returnvalue))))

(event Custom|Attack
  (bind _returnvalue (Game|GetPlayerCharacter 0))
  ;[1 1 1] Attack
  (if (Variables|Default|GetIsThirdAttack)
    (Variables|Default|SetIsThirdAttack false)
    (CallFunction|ResetAttack :!label _label)
    (else
      (bind _result (Math|Integer|IncrementInt (Variables|Default|GetAttackNumber))
        (:%20%20
          (Variables|Default|SetAttackNumber _result)
          (if (== (Variables|Default|GetAttackNumber) 3)
            (goto _label)
            (else
              _))))))
  (Variables|/Script/Engine.CharacterMovementComponent|SetMaxWalkSpeed (Variables|Character|GetCharacterMovement) 1e+02)
  (Variables|Default|SetFacePlayer false)
  (Transformation|SetActorRotation (Math|Rotator|FindLookatRotation (Transformation|GetActorLocation) (Transformation|GetActorLocation _returnvalue)))
  (AI|AIMoveTo self "0, 0, 0" _returnvalue 5.0 false))

(event Custom|PlayerDistance
  ;[1 1 1] PlayerDistance
  (bind _asbp_character (Utilities|Casting|CastToBP_Character (Game|GetPlayerCharacter 0)))
  (bind _output_get (Variables|Default|SetDistanceToPlayer (Math|Vector|VectorLength (- (Transformation|GetActorLocation) (Transformation|GetActorLocation _asbp_character)))))
  (Variables|Default|SetCanAttack (<= _output_get 3e+02)))

(event Custom|ResetAttack
  ;[1 1 1] Attack
  (Variables|Default|SetAttackNumber 0))

(event Custom|PlayerTeleportCheck
  (if (Variables|Default|GetCanTeleport)
    (Variables|Default|SetCanTeleport false)
    (else
      (Variables|Default|SetCanTeleport true))))

(event Custom|Damage
  (bind _sword (Variables|Default|GetSword)
    (:then
      (Default|DoDamage (Utilities|ResolveSoftReference _sword)))
    (:else)))

(event Custom|HitReactRPunchDistance
  (bind _bpcharacter (Variables|Default|GetBPCharacter))
  (bind _capsulecomponent (Variables|Collision|GetCapsuleComponent))
  (Components|MoveComponentTo _capsulecomponent (Transformation|GetWorldLocation (Variables|/Game/Character/BP_Character.BP_Character_C|GetAIHitReactFlyDistance _bpcharacter)) (Math|Rotator|FindLookatRotation (Transformation|GetWorldLocation _capsulecomponent) (Transformation|GetWorldLocation (Variables|/Script/Engine.Character|GetCapsuleComponent _bpcharacter))) false false 1.5 false))

(event Custom|HitLogic
  (bind _healthwidget (Variables|Default|GetHealthWidget))
  (Variables|Default|SetPlayHitAnim true)
  (Rendering|SetVisibility _healthwidget true false)
  (Utilities|FlowControl|Delay 1.0)
  (Rendering|SetVisibility _healthwidget false false))

(event Custom|CheckHit
  (Variables|Default|SetIsHit true)
  (Utilities|FlowControl|Delay 0.2)
  (Variables|Default|SetIsHit false))

(event EventBeginPlay
  (bind _outactors (Actor|GetAllActorsOfClass "/Game/Character/BP_Character.BP_Character_C"))
  (for _array_element _outactors
    ;[1 1 1] AttachWeapon
    (Variables|Default|SetBPCharacter _array_element)
    (Transformation|AttachComponentToComponent (Utilities|ResolveSoftReference (Variables|Default|GetSword)) (Variables|Character|GetMesh) "weapon_r" "SnapToTarget" "SnapToTarget" "SnapToTarget" true)
    (Variables|Default|SetStartHeight (.z (Transformation|GetWorldLocation (Variables|Collision|GetCapsuleComponent))))))

(event EventTick
  (params (DeltaSeconds :type Float%20%28single-precision%29))
  (bind _healthwidget (Variables|Default|GetHealthWidget))
  (Utilities|FlowControl|Sequence
    (:then_0
      (Transformation|SetActorRotation (Math|Rotator|MakeRotator 0.0 0.0 (.Yaw (Math|Rotator|BreakRotator (Transformation|GetWorldRotation (Variables|Collision|GetCapsuleComponent))))))
      (CallFunction|CalculateLaunchHeight))
    (:then_1
      (Transformation|SetWorldRotation _healthwidget (Math|Rotator|FindLookatRotation (Transformation|GetWorldLocation _healthwidget) (Transformation|GetWorldLocation (Variables|/Game/Character/BP_Character.BP_Character_C|GetCamera (Variables|Default|GetBPCharacter)))) false false))))

(fn ConstructionScript)

(fn LevelCheck
  (bind _enemylevel (Variables|Default|GetEnemyLevel))
  (bind _bpcharacter (Variables|Default|GetBPCharacter)
    (:then
      (if (Variables|Default|GetCanCheckLevel)
        (if (not (Variables|/Game/Character/BP_Character.BP_Character_C|GetHighLvlEnemy _bpcharacter))
          (if (> (Variables|/Game/Character/BP_Character.BP_Character_C|GetPlayerLevel _bpcharacter) _enemylevel) :!label _label
            (Development|PrintString "BlueReiatsu")
            (Variables|/Script/Engine.PostProcessComponent|SetbEnabled (Variables|/Game/Character/BP_Character.BP_Character_C|GetReiatsuProcess _bpcharacter) true)
            (Rendering|Material|SetVectorParameterValue (Variables|/Game/Character/BP_Character.BP_Character_C|GetReiatsuMaterial _bpcharacter) "Color" "(R=0.000000,G=0.013314,B=100.000000,A=1.000000)" :!class /Script/Engine.MaterialInstanceDynamic)
            (Audio|PlaySoundatLocation "/Game/Audio/Spiritual_pressure.Spiritual_pressure" (Transformation|GetWorldLocation (Variables|Collision|GetCapsuleComponent)) "0, 0, 0" 1.0 1.0 0.0 0 0 0)
            (elif (== (Variables|/Game/Character/BP_Character.BP_Character_C|GetPlayerLevel _bpcharacter) _enemylevel)
              (Development|PrintString "NoReiatsu")
              (elif (< (Variables|/Game/Character/BP_Character.BP_Character_C|GetPlayerLevel _bpcharacter) _enemylevel)
                (Development|PrintString "RedReiatsu")
                (Variables|/Game/Character/BP_Character.BP_Character_C|SetHighLvlEnemy _bpcharacter true)
                (Variables|/Script/Engine.PostProcessComponent|SetbEnabled (Variables|/Game/Character/BP_Character.BP_Character_C|GetReiatsuProcess _bpcharacter) true)
                (Rendering|Material|SetVectorParameterValue (Variables|/Game/Character/BP_Character.BP_Character_C|GetReiatsuMaterial _bpcharacter) "Color" "(R=100.000000,G=0.000000,B=0.037380,A=1.000000)" :!class /Script/Engine.MaterialInstanceDynamic)
                (Audio|PlaySoundatLocation "/Game/Audio/Spiritual_pressure.Spiritual_pressure" (Transformation|GetWorldLocation (Variables|Collision|GetCapsuleComponent)) "0, 0, 0" 1.0 1.0 0.0 0 0 0)
                (Default|StartEnemyCheck _bpcharacter)
                (else
                  (goto _label)))))
          (return))
        (else
          (Variables|/Script/Engine.PostProcessComponent|SetbEnabled (Variables|/Game/Character/BP_Character.BP_Character_C|GetReiatsuProcess _bpcharacter) false)
          (Rendering|Material|SetVectorParameterValue (Variables|/Game/Character/BP_Character.BP_Character_C|GetReiatsuMaterial _bpcharacter) "Color" "(R=1.000000,G=1.000000,B=1.000000,A=1.000000)" :!class /Script/Engine.MaterialInstanceDynamic)
          (Default|StopEnemyCheck _bpcharacter))))
    (:else)))